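; BP_Item is a pickup item actor that shows its name as world text and displays its assigned static mesh, both set on BeginPlay.
; Its trigger creates a WB_PickUp prompt when the first-person character enters, and hides all top-level instances of that widget on exit without removing them.
; PickUpItem prints a message, returns the Item value and destroys the actor through a short delayed event.
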(event OnComponentBeginOverlap(Trigger)
  (params (OverlappedComponent :type Primitive%20Component%20Object%20Reference) (OtherActor :type Actor%20Object%20Reference) (OtherComp :type Primitive%20Component%20Object%20Reference) (OtherBodyIndex :type Integer) (bFromSweep :type Boolean) (SweepResult :type Hit%20Result%20Structure%20%28by%20ref%29))
  ;[1 1 1] Show/Hide UI
  (Utilities|Casting|CastToBP_FirstPersonCharacter OtherActor)
  (bind _returnvalue (UserInterface|CreateWidget "/Game/Blueprints/Inventory/WB_PickUp.WB_PickUp_C"))
  (UserInterface|Viewport|AddtoViewport _returnvalue 0))

(event OnComponentEndOverlap(Trigger)
  (params (OverlappedComponent :type Primitive%20Component%20Object%20Reference) (OtherActor :type Actor%20Object%20Reference) (OtherComp :type Primitive%20Component%20Object%20Reference) (OtherBodyIndex :type Integer))
  ;[1 1 1] Show/Hide UI
  (Utilities|Casting|CastToBP_FirstPersonCharacter OtherActor)
  (bind _foundwidgets (Widget|GetAllWidgetsOfClass "/Game/Blueprints/Inventory/WB_PickUp.WB_PickUp_C" true))
  (Widget|SetVisibility _foundwidgets "Hidden"))

(event Custom|Destroy%20Item
  ;[1 1 1] Destroy after picking up item
  (Utilities|FlowControl|Delay 0.1)
  (Actor|DestroyActor))

(event EventBeginPlay
  (bind _item_name (Variables|Default|GetItem%20Name))
  ;[1 1 1] Set Text to Item Name and Text Size
  (Rendering|Components|TextRender|SetText _item_name (Utilities|Text|ToText(String) (Variables|Default|GetItem)))
  (Rendering|Components|TextRender|SetWorldSize _item_name (Variables|Default|Get%28Testing%29%20Text%20Size))
  (Components|StaticMesh|SetStaticMesh (Variables|Default|GetModel) (Variables|Default|GetStatic%20Mesh)))

(fn ConstructionScript)

(fn PickUpItem
  (Development|PrintString "Item Picked Up")
  (CallFunction|DestroyItem)
  (return (Variables|Default|GetItem)))